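; Four-arrow rhythm chart editor actor that records and edits notes against a song, optionally at half speed.
; It loads or creates a CSV array of four-digit lines per ~30fps PS1 frame, spawning mesh notes indexed by line.
; A looping timer scrolls notes; arrow keys record during playback, while pausing enables line-by-line selection and toggling.
; Saving on S or EndPlay always writes BambiCSV.txt, whereas loading uses the song's name.
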(event Custom|LineDisplay
  (Development|PrintString (Utilities|String|Append "Current line:" (Utilities|String|ToString(Integer) (Variables|Default|GetActiveCSVLine))) true true "(R=0.000000,G=0.660000,B=1.000000,A=1.000000)" 0.01))

(event Custom|ClearSelection
  (bind _activenotes (Variables|Default|GetActiveNotes))
  (if (> (Utilities|Array|Length _activenotes) 0)
    (for _array_element _activenotes
      (Transformation|SetRelativeScale3D _array_element "0.750000,0.750000,0.750000"))
    (Utilities|Array|Clear (Variables|Default|GetActiveNotes))))

(event Custom|AddNote
  (params (WhichArrow :type Enum_ArrowDirection%20Enum :default "NewEnumerator0"))
  (bind _csvarray (Variables|Default|GetCSVArray))
  (bind _activecsvline (Variables|Default|GetActiveCSVLine))
  (bind _activecsvline_2 (Variables|Default|GetActiveCSVLine))
  (bind _csvarray_2 (Variables|Default|GetCSVArray))
  (bind _output (Utilities|Array|Get(acopy) _csvarray_2 _activecsvline_2))
  (switch Utilities|FlowControl|Switch|SwitchonEnum_ArrowDirection WhichArrow
    (:NewEnumerator0
      (Utilities|Array|SetArrayElem _csvarray _activecsvline (Utilities|String|Append "1" (Utilities|String|GetSubstring _output 1 3))))
    (:NewEnumerator1
      (Utilities|Array|SetArrayElem _csvarray _activecsvline (Utilities|String|Append (Utilities|String|GetSubstring _output 0) "1" (Utilities|String|GetSubstring _output 2 2))))
    (:NewEnumerator2
      (Utilities|Array|SetArrayElem _csvarray _activecsvline (Utilities|String|Append (Utilities|String|GetSubstring _output 0 2) "1" (Utilities|String|GetSubstring _output 3))))
    (:NewEnumerator3
      (Utilities|Array|SetArrayElem _csvarray _activecsvline (Utilities|String|Append (Utilities|String|GetSubstring _output 0 3) "1"))))
  (CallFunction|RebuildLineNotes))

(event Custom|RemoveNote
  (params (WhichArrow :type Enum_ArrowDirection%20Enum :default "NewEnumerator0"))
  (bind _csvarray (Variables|Default|GetCSVArray))
  (bind _activecsvline (Variables|Default|GetActiveCSVLine))
  (bind _csvarray_2 (Variables|Default|GetCSVArray))
  (bind _activecsvline_2 (Variables|Default|GetActiveCSVLine))
  (bind _output (Utilities|Array|Get(acopy) _csvarray _activecsvline))
  (switch Utilities|FlowControl|Switch|SwitchonEnum_ArrowDirection WhichArrow
    (:NewEnumerator0
      (Utilities|Array|SetArrayElem _csvarray_2 _activecsvline_2 (Utilities|String|Append "0" (Utilities|String|GetSubstring _output 1 3))))
    (:NewEnumerator1
      (Utilities|Array|SetArrayElem _csvarray_2 _activecsvline_2 (Utilities|String|Append (Utilities|String|GetSubstring _output 0) "0" (Utilities|String|GetSubstring _output 2 2))))
    (:NewEnumerator2
      (Utilities|Array|SetArrayElem _csvarray_2 _activecsvline_2 (Utilities|String|Append (Utilities|String|GetSubstring _output 0 2) "0" (Utilities|String|GetSubstring _output 3))))
    (:NewEnumerator3
      (Utilities|Array|SetArrayElem _csvarray_2 _activecsvline_2 (Utilities|String|Append (Utilities|String|GetSubstring _output 0 3) "0"))))
  (CallFunction|RebuildLineNotes))

(event Custom|UpdateEditingLine
  (bind _selectionline (Variables|Default|GetSelectionLine))
  (bind _returnvalue (Transformation|GetWorldLocation _selectionline))
  (Transformation|SetWorldLocation _selectionline (Math|Vector|MakeVector (.x _returnvalue) (.y _returnvalue) (CallFunction|CSVLinetoWorldZ)) false false))

(event Custom|OneLineScroll
  (params (IsUp :type Boolean))
  (bind _activecsvline (Variables|Default|GetActiveCSVLine))
  (if IsUp
    (CallFunction|ClearSelection)
    (bind _result (Math|Integer|IncrementInt _activecsvline)
      (:%20%20
        (CallFunction|UpdateEditingLine)
        (if (.ReturnValue (Utilities|Map|Find (Variables|Default|GetCSVToNotesMap) _result))
          (for _array_element (Utilities|Struct|BreakBPS_LineData (.Value (Utilities|Map|Find (Variables|Default|GetCSVToNotesMap) _result)))
            (Utilities|Array|Add (Variables|Default|GetActiveNotes) (Utilities|Array|Get(acopy) (Variables|Default|GetNotes) _array_element))
            (Transformation|SetRelativeScale3D (Utilities|Array|Get(acopy) (Variables|Default|GetNotes) _array_element) "0.850000,0.850000,0.850000")))))
    (else
      (CallFunction|ClearSelection)
      (bind _result_2 (Math|Integer|DecrementInt _activecsvline)
        (:%20%20
          (CallFunction|UpdateEditingLine)
          (if (.ReturnValue (Utilities|Map|Find (Variables|Default|GetCSVToNotesMap) _result_2))
            (for _array_element_2 (Utilities|Struct|BreakBPS_LineData (.Value (Utilities|Map|Find (Variables|Default|GetCSVToNotesMap) _result_2)))
              (Utilities|Array|Add (Variables|Default|GetActiveNotes) (Utilities|Array|Get(acopy) (Variables|Default|GetNotes) _array_element_2))
              (Transformation|SetRelativeScale3D (Utilities|Array|Get(acopy) (Variables|Default|GetNotes) _array_element_2) "0.850000,0.850000,0.850000"))))))))

(event Custom|TimerTick
  (bind _returnvalue (Utilities|Time|GetGameTimeinSeconds))
  (bind _speed (Variables|Default|GetSpeed))
  (if (Variables|Default|GetIsHalfSpeed)
    (Utilities|FlowControl|FlipFlop
      (:A
        _)
      (:B
        (Math|Integer|IncrementInt (Variables|Default|GetFrameCount) :!label _label
          (:%20%20
            _))))
    (else
      (goto _label)))
  (for _array_element (Variables|Default|GetNotes)
    (Utilities|IsValid _array_element
      (:Is%20Valid
        (Transformation|SetWorldLocation _array_element (Math|Vector|MakeVector (.x (Transformation|GetWorldLocation _array_element)) (.y (Transformation|GetWorldLocation _array_element)) (- (.z (Transformation|GetWorldLocation _array_element)) (Math|Float|SelectFloat (* _speed 0.5) _speed (Variables|Default|GetIsHalfSpeed)))) false false))))
  (Development|PrintString (Utilities|String|ToString(Float) (- _returnvalue (stale _output_get))) (or (> (- _returnvalue (stale _output_get)) 0.0335) (< (- _returnvalue (stale _output_get)) 0.033)) (or (> (- _returnvalue (stale _output_get)) 0.0335) (< (- _returnvalue (stale _output_get)) 0.033))) ; timer safety check
  (bind _output_get (Variables|Default|Setlast%20frame%20time _returnvalue)))

(event EventBeginPlay
  (bind _song (Variables|Default|GetSong))
  (bind _csvtonotesmap (Variables|Default|GetCSVToNotesMap))
  (bind _sound (Variables|/Script/Engine.AudioComponent|GetSound _song))
  (bind _returnvalue (Utilities|GetDisplayName _sound))
  (Audio|Components|Audio|SetPitchMultiplier (Variables|Default|GetSong) (Math|Float|SelectFloat 0.5 1.0 (Variables|Default|GetIsHalfSpeed)))
  (bind (_result _returnvalue_2) (Class|VictoryBPFunctionLibrary|LoadStringfromFile (Utilities|String|Append "C:\\Users\\rwk_n\\Documents\\Unreal Projects\\NoteChartBuilder\\Content" "\\" _returnvalue "CSV.txt")))
  (if _returnvalue_2
    (Development|PrintString (Utilities|String|Append "Loaded " _returnvalue "CSV.txt"))
    (Variables|Default|SetCSVArray (Utilities|String|ParseIntoArray _result ","))
    ;[1 1 1] make notes from csv entry
    (for (_array_element _array_index) (Utilities|String|ParseIntoArray _result ",")
      (if (Utilities|Enum|NotEqual(Enum) _array_element "0000")
        (for _index (range 0 3)
          (if (Math|Conversions|ToBoolean(Integer) (Math|Conversions|ToInteger(Byte) (Utilities|String|GetSubstring _array_element _index)))
            (bind _returnvalue_3 (AddComponent|AddStaticMeshComponent false (Math|Transform|MakeTransform (Math|Vector|MakeVector (Utilities|Select :Index _index :Option%200 125.0 :Option%201 42.0 :Option%202 -42.0 :Option%203 -125.0) -0.5 0.0) (Math|Rotator|MakeRotator 9e+01 (Utilities|Select :Index _index :Option%200 0.0 :Option%201 9e+01 :Option%202 -9e+01 :Option%203 1.8e+02) 1.8e+02) "0.750000,0.750000,0.750000")))
            (bind _returnvalue_4 (Utilities|Array|Add (Variables|Default|GetNotes) _returnvalue_3))
            (if (.ReturnValue (Utilities|Map|Find _csvtonotesmap _array_index)) ; create new map entry if not found, if found just add the note index to the data in the map
              (bind _output_get (Variables|Default|SetTempArray (Utilities|Struct|BreakBPS_LineData (.Value (Utilities|Map|Find _csvtonotesmap _array_index)))))
              (Utilities|Array|Add _output_get _returnvalue_4)
              (Utilities|Map|Add _csvtonotesmap _array_index (Utilities|Struct|MakeBPS_LineData _output_get))
              (else
                (Utilities|Map|Add _csvtonotesmap _array_index (Utilities|Struct|MakeBPS_LineData (Utilities|Array|MakeArray _returnvalue_4)))))
            (Transformation|SetWorldLocation _returnvalue_3 (Math|Vector|MakeVector (.x (Transformation|GetWorldLocation _returnvalue_3)) (.y (Transformation|GetWorldLocation _returnvalue_3)) (+ (.z (Transformation|GetWorldLocation _returnvalue_3)) (* _array_index (Variables|Default|GetSpeed)) (Variables|Default|GetStartOffset))) false false)))
        (Utilities|Array|Clear (Variables|Default|GetTempArray))))
    (else
      (Development|PrintString (Utilities|String|Append "Couldn't load " _returnvalue "CSV.txt, creating new blank CSV array"))
      ;[1 1 1] create new array if none found
      (for _index_2 (range 0 (Math|Float|Round (* (Variables|/Script/Engine.SoundBase|GetDuration (Variables|/Script/Engine.AudioComponent|GetSound (Variables|Default|GetSong))) 29.913)))
        (Utilities|Array|Add (Variables|Default|GetCSVArray) "0000"))
      (Development|PrintString (Utilities|String|ToString(Integer) (Utilities|Array|Length (Variables|Default|GetCSVArray))))))
  (Utilities|FlowControl|Delay 2.0)
  (Audio|Components|Audio|Play (Variables|Default|GetSong) 0.0)
  (bind _returnvalue_5 (Utilities|Time|SetTimerbyEvent (delegate Custom|TimerTick) 0.03343 true)) ; PS1's NTSC 30fps frame time
  (Variables|Default|SetTickyTimer _returnvalue_5)
  (Actor|Tick|SetActorTickEnabled true)
  (Utilities|Time|SetTimerbyEvent (delegate Custom|LineDisplay) 0.033 true) ; display currently selected line, use for editing CSV manually
)

(event Collision|EventActorBeginOverlap
  (params (OtherActor :type Actor%20Object%20Reference)))

(event EventEndPlay
  (params (EndPlayReason :type EEndPlayReason%20Enum :default "Destroyed"))
  (Class|VictoryBPFunctionLibrary|FileIOSaveStringTexttoFile "C:\\Users\\rwk_n\\Documents\\Unreal Projects\\NoteChartBuilder\\Content" "BambiCSV.txt" (Utilities|String|JoinStringArray (Variables|Default|GetCSVArray) ",") true false))

(event Input|KeyboardEvents|SpaceBar
  (params (Key :type Key%20Structure :default "None"))
  (bind _song (Variables|Default|GetSong))
  (bind _tickytimer (Variables|Default|GetTickyTimer))
  (bind _activenotes (Variables|Default|GetActiveNotes))
  (bind _selectionline (Variables|Default|GetSelectionLine))
  (:Pressed
    (Utilities|FlowControl|FlipFlop
      (:A
        (Class|AudioComponent|SetPaused _song true)
        (Utilities|Time|PauseTimerbyHandle _tickytimer)
        (Actor|Tick|SetActorTickEnabled false)
        (Development|SetHiddeninGame _selectionline false false)
        (bind _index (Utilities|FlowControl|ForLoopwithBreak (- (Variables|Default|GetFrameCount) 10) (Utilities|Array|Length (Variables|Default|GetCSVArray)) :!label _label)
          (:LoopBody
            (if (.ReturnValue (Utilities|Map|Find (Variables|Default|GetCSVToNotesMap) _index))
              (Variables|Default|SetActiveCSVLine _index)
              (for _array_element (Utilities|Struct|BreakBPS_LineData (.Value (Utilities|Map|Find (Variables|Default|GetCSVToNotesMap) _index)))
                (Utilities|Array|Add (Variables|Default|GetActiveNotes) (Utilities|Array|Get(acopy) (Variables|Default|GetNotes) _array_element))
                (Transformation|SetRelativeScale3D (Utilities|Array|Get(acopy) (Variables|Default|GetNotes) _array_element) "0.850000,0.850000,0.850000"))
              (goto _label Break)))
          (:Completed
            (CallFunction|UpdateEditingLine))))
      (:B
        (Class|AudioComponent|SetPaused _song false)
        (Utilities|Time|UnpauseTimerbyHandle _tickytimer)
        (Actor|Tick|SetActorTickEnabled true)
        (Development|SetHiddeninGame _selectionline true false)
        (if (> (Utilities|Array|Length _activenotes) 0)
          (for _array_element_2 _activenotes
            (Transformation|SetRelativeScale3D _array_element_2 "0.750000,0.750000,0.750000"))
          (Utilities|Array|Clear (Variables|Default|GetActiveNotes)))))))

(event Input|KeyboardEvents|Left
  (params (Key :type Key%20Structure :default "None"))
  (:Pressed
    (if (Class|Actor|IsActorTickEnabled)
      (Variables|Default|SetActiveCSVLine (Variables|Default|GetFrameCount))
      (CallFunction|AddNote "NewEnumerator0"))))

(event Input|KeyboardEvents|2
  (params (Key :type Key%20Structure :default "None"))
  (:Pressed
    (if (not (Class|Actor|IsActorTickEnabled))
      (if (Utilities|Enum|Equal(Enum) (Utilities|String|GetSubstring (Utilities|Array|Get(acopy) (Variables|Default|GetCSVArray) (Variables|Default|GetActiveCSVLine)) 1) "0")
        (CallFunction|AddNote "NewEnumerator1")
        (else
          (CallFunction|RemoveNote "NewEnumerator1"))))))

(event Input|KeyboardEvents|3
  (params (Key :type Key%20Structure :default "None"))
  (:Pressed
    (if (not (Class|Actor|IsActorTickEnabled))
      (if (Utilities|Enum|Equal(Enum) (Utilities|String|GetSubstring (Utilities|Array|Get(acopy) (Variables|Default|GetCSVArray) (Variables|Default|GetActiveCSVLine)) 2) "0")
        (CallFunction|AddNote "NewEnumerator2")
        (else
          (CallFunction|RemoveNote "NewEnumerator2"))))))

(event Input|KeyboardEvents|4
  (params (Key :type Key%20Structure :default "None"))
  (:Pressed
    (if (not (Class|Actor|IsActorTickEnabled))
      (if (Utilities|Enum|Equal(Enum) (Utilities|String|GetSubstring (Utilities|Array|Get(acopy) (Variables|Default|GetCSVArray) (Variables|Default|GetActiveCSVLine)) 3) "0")
        (CallFunction|AddNote "NewEnumerator3")
        (else
          (CallFunction|RemoveNote "NewEnumerator3"))))))

(event Input|KeyboardEvents|Z
  (params (Key :type Key%20Structure :default "None"))
  ;[1 1 1] skip back
  (:Pressed
    (if (not (Class|KismetSystemLibrary|IsTimerPausedHandle (Variables|Default|GetTickyTimer)))
      (bind _output_get (Variables|Default|SetFrameCount (- (Variables|Default|GetFrameCount) 60)))
      (Audio|Components|Audio|Play (Variables|Default|GetSong) (* _output_get 0.03343))
      (for _array_element (Variables|Default|GetNotes)
        (Utilities|IsValid _array_element
          (:Is%20Valid
            (Transformation|SetWorldLocation _array_element (Math|Vector|MakeVector (.x (Transformation|GetWorldLocation _array_element)) (.y (Transformation|GetWorldLocation _array_element)) (+ (.z (Transformation|GetWorldLocation _array_element)) (* (Variables|Default|GetSpeed) 6e+01))) false false)))))))

(event Input|KeyboardEvents|X
  (params (Key :type Key%20Structure :default "None"))
  ;[1 1 1] skip forward
  (:Pressed
    (if (not (Class|KismetSystemLibrary|IsTimerPausedHandle (Variables|Default|GetTickyTimer)))
      (bind _output_get (Variables|Default|SetFrameCount (+ (Variables|Default|GetFrameCount) 60)))
      (Audio|Components|Audio|Play (Variables|Default|GetSong) (* _output_get 0.03343))
      (for _array_element (Variables|Default|GetNotes)
        (Utilities|IsValid _array_element
          (:Is%20Valid
            (Transformation|SetWorldLocation _array_element (Math|Vector|MakeVector (.x (Transformation|GetWorldLocation _array_element)) (.y (Transformation|GetWorldLocation _array_element)) (- (.z (Transformation|GetWorldLocation _array_element)) (* (Variables|Default|GetSpeed) 6e+01))) false false)))))))

(event Input|KeyboardEvents|S
  (params (Key :type Key%20Structure :default "None"))
  (:Pressed
    (Class|VictoryBPFunctionLibrary|FileIOSaveStringTexttoFile "C:\\Users\\rwk_n\\Documents\\Unreal Projects\\NoteChartBuilder\\Content" "BambiCSV.txt" (Utilities|String|JoinStringArray (Variables|Default|GetCSVArray) ",") true false)))

(event Input|KeyboardEvents|PageUp
  (params (Key :type Key%20Structure :default "None"))
  (:Pressed
    (bind _index (Utilities|FlowControl|ForLoopwithBreak (+ (Variables|Default|GetActiveCSVLine) 1) (Utilities|Array|Length (Variables|Default|GetCSVArray)) :!label _label)
      (:LoopBody
        (if (.ReturnValue (Utilities|Map|Find (Variables|Default|GetCSVToNotesMap) _index))
          (CallFunction|ClearSelection)
          (Variables|Default|SetActiveCSVLine _index)
          (for _array_element (Utilities|Struct|BreakBPS_LineData (.Value (Utilities|Map|Find (Variables|Default|GetCSVToNotesMap) _index)))
            (Utilities|Array|Add (Variables|Default|GetActiveNotes) (Utilities|Array|Get(acopy) (Variables|Default|GetNotes) _array_element))
            (Transformation|SetRelativeScale3D (Utilities|Array|Get(acopy) (Variables|Default|GetNotes) _array_element) "0.850000,0.850000,0.850000"))
          (goto _label Break)))
      (:Completed
        (CallFunction|UpdateEditingLine)))))

(event Input|KeyboardEvents|PageDown
  (params (Key :type Key%20Structure :default "None"))
  (:Pressed
    (bind _index (Utilities|BetterforLoop (- (Variables|Default|GetActiveCSVLine) 1) "NewEnumerator3" (- (Variables|Default|GetActiveCSVLine) 300))
      (:Loop%20Body
        (if (not (Variables|Default|GetLowNoteFound))
          (if (.ReturnValue (Utilities|Map|Find (Variables|Default|GetCSVToNotesMap) _index))
            (CallFunction|ClearSelection)
            (Variables|Default|SetActiveCSVLine _index)
            (Variables|Default|SetLowNoteFound true)
            (for _array_element (Utilities|Struct|BreakBPS_LineData (.Value (Utilities|Map|Find (Variables|Default|GetCSVToNotesMap) _index)))
              (Utilities|Array|Add (Variables|Default|GetActiveNotes) (Utilities|Array|Get(acopy) (Variables|Default|GetNotes) _array_element))
              (Transformation|SetRelativeScale3D (Utilities|Array|Get(acopy) (Variables|Default|GetNotes) _array_element) "0.850000,0.850000,0.850000")))))
      (:Completed
        (Variables|Default|SetLowNoteFound false)
        (CallFunction|UpdateEditingLine)))))

(event Input|KeyboardEvents|R
  (params (Key :type Key%20Structure :default "None"))
  (:Pressed
    (Utilities|FlowControl|FlipFlop
      (:A
        (Variables|Default|SetRecordMode true)
        (Development|PrintString "Record Mode On"))
      (:B
        (Variables|Default|SetRecordMode false)
        (Development|PrintString "Record Mode Off")))))

(event Input|KeyboardEvents|Down
  (params (Key :type Key%20Structure :default "None"))
  (:Pressed
    (if (Class|Actor|IsActorTickEnabled)
      (Variables|Default|SetActiveCSVLine (Variables|Default|GetFrameCount))
      (CallFunction|AddNote "NewEnumerator1")
      (else
        (CallFunction|OneLineScroll false)))))

(event Input|KeyboardEvents|Up
  (params (Key :type Key%20Structure :default "None"))
  (:Pressed
    (if (Class|Actor|IsActorTickEnabled)
      (Variables|Default|SetActiveCSVLine (Variables|Default|GetFrameCount))
      (CallFunction|AddNote "NewEnumerator2")
      (else
        (CallFunction|OneLineScroll true)))))

(event Input|KeyboardEvents|Right
  (params (Key :type Key%20Structure :default "None"))
  (:Pressed
    (if (Class|Actor|IsActorTickEnabled)
      (Variables|Default|SetActiveCSVLine (Variables|Default|GetFrameCount))
      (CallFunction|AddNote "NewEnumerator3"))))

(event Input|KeyboardEvents|1
  (params (Key :type Key%20Structure :default "None"))
  (:Pressed
    (if (not (Class|Actor|IsActorTickEnabled))
      (if (Utilities|Enum|Equal(Enum) (Utilities|String|GetSubstring (Utilities|Array|Get(acopy) (Variables|Default|GetCSVArray) (Variables|Default|GetActiveCSVLine)) 0) "0")
        (CallFunction|AddNote "NewEnumerator0")
        (else
          (CallFunction|RemoveNote "NewEnumerator0"))))))

(fn ConstructionScript)

(fn CSVLinetoWorldZ
  (return (- (+ (* (Variables|Default|GetActiveCSVLine) (Variables|Default|GetSpeed)) (+ (.z (Transformation|GetActorLocation)) (Variables|Default|GetStartOffset))) (* (Variables|Default|GetFrameCount) (Variables|Default|GetSpeed)))))

(fn RebuildLineNotes
  (bind _activenotes (Variables|Default|GetActiveNotes))
  (bind _csvtonotesmap (Variables|Default|GetCSVToNotesMap))
  (bind _activecsvline (Variables|Default|GetActiveCSVLine))
  (bind (_value _returnvalue) (Utilities|Map|Find _csvtonotesmap _activecsvline))
  (for _array_element _activenotes
    (Utilities|IsValid _array_element
      (:Is%20Valid
        (Components|DestroyComponent _array_element))))
  (Utilities|Array|Clear _activenotes)
  (Utilities|Map|Remove (Variables|Default|GetCSVToNotesMap) (Variables|Default|GetActiveCSVLine))
  (for _index (range 0 3)
    (if (Math|Conversions|ToBoolean(Integer) (Math|Conversions|ToInteger(Byte) (Utilities|String|GetSubstring (Utilities|Array|Get(acopy) (Variables|Default|GetCSVArray) (Variables|Default|GetActiveCSVLine)) _index)))
      (bind _returnvalue_2 (AddComponent|AddStaticMeshComponent false (Math|Transform|MakeTransform (Math|Vector|MakeVector (Utilities|Select :Index _index :Option%200 125.0 :Option%201 42.0 :Option%202 -42.0 :Option%203 -125.0) -3.0 0.0) (Math|Rotator|MakeRotator 9e+01 (Utilities|Select :Index _index :Option%200 0.0 :Option%201 9e+01 :Option%202 -9e+01 :Option%203 1.8e+02) 1.8e+02) "0.850000,0.850000,0.850000")))
      (bind _returnvalue_3 (Utilities|Array|Add (Variables|Default|GetNotes) _returnvalue_2))
      (Utilities|Array|Add (Variables|Default|GetActiveNotes) _returnvalue_2)
      (if _returnvalue ; create new map entry if not found, if found just add the note index to the data in the map
        (bind _output_get (Variables|Default|SetTempArray (Utilities|Struct|BreakBPS_LineData _value)))
        (Utilities|Array|Add _output_get _returnvalue_3)
        (Utilities|Map|Add _csvtonotesmap _activecsvline (Utilities|Struct|MakeBPS_LineData _output_get))
        (else
          (Utilities|Map|Add _csvtonotesmap _activecsvline (Utilities|Struct|MakeBPS_LineData (Utilities|Array|MakeArray _returnvalue_3)))))
      (Transformation|SetWorldLocation _returnvalue_2 (Math|Vector|MakeVector (.x (Transformation|GetWorldLocation _returnvalue_2)) (.y (Transformation|GetWorldLocation _returnvalue_2)) (CallFunction|CSVLinetoWorldZ)) false false)))
  (Utilities|Array|Clear (Variables|Default|GetTempArray)))